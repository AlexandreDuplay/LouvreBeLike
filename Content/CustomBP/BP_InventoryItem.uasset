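; BP_InventoryItem is an interactable world pickup that hands its item to the first-person character.
; On Interact, it passes its ItemID to the character's ItemHasBeenPickedUp, then messages the ScoreController, plays a pickup sound and destroys itself.
; Items flagged as Diamond also set HasDiamond on the Reftotimer of each first-person character, with the score, sound and destroy steps running inside that loop.
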(event EventInteract
  (params (ActorTriggeringInteract :type Actor%20Object%20Reference))
  (bind _asbp_first_person_character (Utilities|Casting|CastToBP_FirstPersonCharacter ActorTriggeringInteract))
  (Default|ItemHasBeenPickedUp _asbp_first_person_character (Variables|Default|GetItem%20ID))
  (if (Variables|Default|Getdiamond)
    (bind _outactors (Actor|GetAllActorsOfClass "/Game/FirstPerson/Blueprints/BP_FirstPersonCharacter.BP_FirstPersonCharacter_C"))
    (for _array_element _outactors
      (Variables|/Game/CustomBP/timer.timer_C|SetHas%20diamond (Variables|/Game/FirstPerson/Blueprints/BP_FirstPersonCharacter.BP_FirstPersonCharacter_C|Getreftotimer _array_element) true)
      (Class|BPIPlayerAction|Interact(Message) (Variables|Default|GetScoreController) self)
      (Audio|PlaySoundatLocation "/Game/Sounds/ItemPickUp.ItemPickUp" "0, 0, 0" "0, 0, 0" 1.0 1.0 0.0 0 0 0 0)
      (Actor|DestroyActor))
    (else
      (Class|BPIPlayerAction|Interact(Message) (Variables|Default|GetScoreController) self)
      (Audio|PlaySoundatLocation "/Game/Sounds/ItemPickUp.ItemPickUp" "0, 0, 0" "0, 0, 0" 1.0 1.0 0.0 0 0 0 0)
      (Actor|DestroyActor))))

(fn ConstructionScript
  (|CallParentFunction))