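; Rotatable statue pillar for a puzzle, turned through Interact while IsPlayerInteractable is set.
; Each interaction rotates the Cube by a quarter turn derived from its world rotation, carrying Childf, which is attached at BeginPlay.
; If the resulting yaw lies between MinAngle and MaxAngle, it unlocks Childf, otherwise it locks it, casting to Bell, BronzeObject or Crown.
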(event EventBeginPlay
  (Transformation|AttachComponentToComponent (Variables|Default|Getchildf) (Variables|Default|GetCube) "None" "KeepWorld" "KeepRelative" "KeepRelative" true))

(event EventInteract
  (params (ActorTriggeringInteract :type Actor%20Object%20Reference))
  (bind _isplayerinteractable (Variables|Default|GetIsPlayerInteractable))
  (bind _cube (Variables|Default|GetCube))
  (bind _returnvalue (Transformation|GetWorldRotation _cube))
  (bind _yaw (Math|Rotator|BreakRotator _returnvalue))
  (Utilities|Casting|CastToBP_FirstPersonCharacter ActorTriggeringInteract
    (:then
      (if _isplayerinteractable
        (Transformation|SetRelativeRotation (Variables|Default|GetCube) (Math|Conversions|RotationFromXVector (Math|Vector|RotateVector "0.000000,90.000000,0.000000" (Transformation|GetWorldRotation (Variables|Default|GetCube)))) false false :!label _label)
        (Development|PrintString (Utilities|String|ToString(Float) _yaw))
        (if (and (<= _yaw (Variables|Default|GetmaxAngle)) (>= (.Yaw (Math|Rotator|BreakRotator (Transformation|GetWorldRotation (Variables|Default|GetCube)))) (Variables|Default|GetminAngle)))
          (Development|PrintString "unlock")
          (bind _asbp_bell (Utilities|Casting|CastToBP_Bell (Variables|Default|Getchildf))
            (:then
              (Default|Unlock _asbp_bell))
            (:CastFailed
              (bind _asbp_bronze_object (Utilities|Casting|CastToBP_BronzeObject (Variables|Default|Getchildf))
                (:then
                  (Default|Unlock _asbp_bronze_object))
                (:CastFailed
                  (bind _asbp_crown (Utilities|Casting|CastToBP_Crown (Variables|Default|Getchildf)))
                  (Default|Unlock _asbp_crown)))))
          (else
            (Development|PrintString "lock")
            (bind _asbp_bell_2 (Utilities|Casting|CastToBP_Bell (Variables|Default|Getchildf))
              (:then
                (Default|Lock _asbp_bell_2))
              (:CastFailed
                (bind _asbp_bronze_object_2 (Utilities|Casting|CastToBP_BronzeObject (Variables|Default|Getchildf))
                  (:then
                    (Default|Lock _asbp_bronze_object_2))
                  (:CastFailed
                    (bind _asbp_crown_2 (Utilities|Casting|CastToBP_Crown (Variables|Default|Getchildf)))
                    (Default|Lock _asbp_crown_2)))))))))
    (:CastFailed
      (if _isplayerinteractable
        (goto _label)))))

(fn ConstructionScript)