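; Interactable platform that slides between two target points, alternating on each use via a FlipFlop over a timed MoveComponentTo.
; IsPlayerCharacterInteractable decides whether the first-person player or only other actors can trigger it.
; An optional item lock checks the player's inventory and can consume the items; unlocking plays a sound without moving the platform.
; IsOpenedAtStart runs the first move on BeginPlay, and each move updates the look-at action name.
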(event EventInteract
  (params (ActorTriggeringInteract :type Actor%20Object%20Reference))
  (bind _isplayercharacterinteractable (Variables|Default|GetisPlayerCharacterInteractable))
  (bind _asbp_first_person_character (Utilities|Casting|CastToBP_FirstPersonCharacter ActorTriggeringInteract)
    (:then
      (if _isplayercharacterinteractable
        (if (Variables|Default|GetisItemNeeded) :!label _label
          (if (.ReturnValue (Utilities|Map|Find (Variables|/Game/FirstPerson/Blueprints/BP_FirstPersonCharacter.BP_FirstPersonCharacter_C|GetInventory _asbp_first_person_character) (Variables|Default|GetItem%20ID)))
            (if (>= (.Value (Utilities|Map|Find (Variables|/Game/FirstPerson/Blueprints/BP_FirstPersonCharacter.BP_FirstPersonCharacter_C|GetInventory _asbp_first_person_character) (Variables|Default|GetItem%20ID))) (Variables|Default|GetAmountOfItemsNeeded))
              (Variables|Default|SetisItemNeeded false)
              (Audio|PlaySoundatLocation "/Game/Audio/key-insertion-100575.key-insertion-100575" (Transformation|GetActorLocation) "0, 0, 0" 1.0 1.0 0.0 0 0 0 0)
              (if (Variables|Default|GetisItemRemoved)
                (Utilities|Map|Add (Variables|/Game/FirstPerson/Blueprints/BP_FirstPersonCharacter.BP_FirstPersonCharacter_C|GetInventory _asbp_first_person_character) (Variables|Default|GetItem%20ID) (- (.Value (Utilities|Map|Find (Variables|/Game/FirstPerson/Blueprints/BP_FirstPersonCharacter.BP_FirstPersonCharacter_C|GetInventory _asbp_first_person_character) (Variables|Default|GetItem%20ID))) (Variables|Default|GetAmountOfItemsNeeded))))
              (if (stale _isa)
                (Variables|Default|SetLookAtActionName (Variables|Default|GetActionNameForA))
                (else
                  (Variables|Default|SetLookAtActionName (Variables|Default|GetActionNameForB))))))
          (else
            (Audio|PlaySoundatLocation "/Game/Sounds/ElectricalLader.ElectricalLader" "0, 0, 0" "0, 0, 0" 1.0 1.0 0.0 0 0 0 0)
            (bind _isa (Utilities|FlowControl|FlipFlop)
              (:A
                (Variables|Default|SetLookAtActionName (Variables|Default|GetActionNameForA))
                (Components|MoveComponentTo (Variables|Default|GetPlatform) (Math|Transform|TransformLocation (Transformation|GetRelativeTransform (Variables|Default|GetTarget)) "0, 0, 0") "0, 0, 0" false false 2.0 false))
              (:B
                (Variables|Default|SetLookAtActionName (Variables|Default|GetActionNameForB))
                (Components|MoveComponentTo (Variables|Default|GetPlatform) (Math|Transform|TransformLocation (Transformation|GetRelativeTransform (Variables|Default|GetTarget1)) "0, 0, 0") "0, 0, 0" false false 2.0 false)))))))
    (:CastFailed
      (if (not _isplayercharacterinteractable)
        (goto _label)))))

(event EventBeginPlay
  (if (Variables|Default|GetisOpenedAtStart)
    (Audio|PlaySoundatLocation "/Game/Sounds/ElectricalLader.ElectricalLader" "0, 0, 0" "0, 0, 0" 1.0 1.0 0.0 0 0 0 0)
    (bind _isa (Utilities|FlowControl|FlipFlop)
      (:A
        (Variables|Default|SetLookAtActionName (Variables|Default|GetActionNameForA))
        (Components|MoveComponentTo (Variables|Default|GetPlatform) (Math|Transform|TransformLocation (Transformation|GetRelativeTransform (Variables|Default|GetTarget)) "0, 0, 0") "0, 0, 0" false false 2.0 false))
      (:B
        (Variables|Default|SetLookAtActionName (Variables|Default|GetActionNameForB))
        (Components|MoveComponentTo (Variables|Default|GetPlatform) (Math|Transform|TransformLocation (Transformation|GetRelativeTransform (Variables|Default|GetTarget1)) "0, 0, 0") "0, 0, 0" false false 2.0 false)))))

(fn ConstructionScript
  (|CallParentFunction))